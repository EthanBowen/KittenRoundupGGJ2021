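; Day-night cycle Blueprint that rotates the Sun and Moon over a configurable day length.
; On BeginPlay it scales the WorldTime timeline's play rate by DayLength.
; Each timeline update sets sun pitch, offsets the moon by 180 degrees and keeps both actors' initial sun roll and yaw.
; It also writes SunRotation to the PP_Params material parameter collection and refreshes the sky sphere's sun direction.
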(event `self.ReceiveBeginPlay`
  (bind _skysphere (`self.SkySphere`))
  (bind _roll (.roll (`self.InitialRotation`)))
  (bind _yaw (.yaw (`self.InitialRotation`)))
  (set `self.InitialRotation` (`self.K2_GetActorRotation` (`self.Sun`)))
  (`TimelineComponent.SetPlayRate` (`self.WorldTime`) (/ 1.0 (* 120 (`self.DayLength`))))
  (bind (_direction _sunpitch) (`Timeline|WorldTime` :`NewTime` 0.55 :!via `SetNewTime`)
    (:`Update`
      (`KismetMaterialLibrary.SetScalarParameterValue` "/Game/Materials/PP_Params.PP_Params" "SunRotation" _sunpitch)
      (`self.K2_SetActorRotation` (`self.Sun`) (`KismetMathLibrary.MakeRotator` _roll _sunpitch _yaw) false)
      (`self.K2_SetActorRotation` (`self.Moon`) (`KismetMathLibrary.MakeRotator` _roll (+ _sunpitch 180.0) _yaw) false)
      (set `/Game/BP_Sky_Sphere_Stylized.Refresh material` true _skysphere)
      (`/Game/BP_Sky_Sphere_Stylized.UpdateSunDirection` _skysphere))))

(fn `NewFunction_0`)

(fn `UserConstructionScript`)